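; Example actor that builds a single colored triangle with the Realtime Mesh Component plugin.
; The construction script chains a mesh builder through three red, green and blue vertices with normals and UVs, then adds two opposite-winding triangles over them so both sides render.
; It initializes a RealtimeMeshSimple and creates a named LOD 0 section group from that data.
; The event graph is unused.
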(event EventBeginPlay)

(event Collision|EventActorBeginOverlap
  (params (OtherActor :type Actor%20Object%20Reference)))

(event EventTick
  (params (DeltaSeconds :type Float%20%28single-precision%29)))

(fn ConstructionScript
  (bind _returnvalue (Class|RealtimeMeshActor|MakeMeshBuilder "Normal" "Normal" false "None" true 1 true))
  (bind _builder (Class|RealtimeMeshLocalBuilder|AddVertex _returnvalue (Utilities|Struct|MakeRealtimeMeshBasicVertex "-50.000000,0.000000,0.000000" "0.000000,-1.000000,0.000000" "1.000000,0.000000,0.000000" "0.000000,1.000000,0.000000" "(R=1.000000,G=0.000000,B=0.000000,A=1.000000)" "(X=0.000000,Y=1.000000)" "(X=0.000000,Y=0.000000)" "(X=0.000000,Y=0.000000)" "(X=0.000000,Y=0.000000)")))
  (bind _builder_2 (Class|RealtimeMeshLocalBuilder|AddVertex _builder (Utilities|Struct|MakeRealtimeMeshBasicVertex "0.000000,0.000000,100.000000" "0.000000,-1.000000,0.000000" "1.000000,0.000000,0.000000" "0.000000,1.000000,0.000000" "(R=0.000000,G=1.000000,B=0.000000,A=1.000000)" "(X=0.500000,Y=0.000000)" "(X=0.000000,Y=0.000000)" "(X=0.000000,Y=0.000000)" "(X=0.000000,Y=0.000000)")))
  (bind _builder_3 (Class|RealtimeMeshLocalBuilder|AddVertex _builder_2 (Utilities|Struct|MakeRealtimeMeshBasicVertex "50.000000,0.000000,0.000000" "0.000000,-1.000000,0.000000" "1.000000,0.000000,0.000000" "0.000000,1.000000,0.000000" "(R=0.000000,G=0.000000,B=1.000000,A=1.000000)" "(X=1.000000,Y=1.000000)" "(X=0.000000,Y=0.000000)" "(X=0.000000,Y=0.000000)" "(X=0.000000,Y=0.000000)")))
  (bind _builder_4 (Class|RealtimeMeshLocalBuilder|AddTriangle _builder_3 0 1 2))
  (bind _builder_5 (Class|RealtimeMeshLocalBuilder|AddTriangle _builder_4 2 1))
  (bind _returnvalue_2 (Class|RealtimeMeshComponent|InitializeRealtimeMesh (Variables|Default|GetRealtimeMeshComponent) "/Script/RealtimeMeshComponent.RealtimeMeshSimple"))
  (Class|RealtimeMeshSimple|CreateSectionGroup _returnvalue_2 (Class|RealtimeMeshBlueprintFunctionLibrary|MakeSectionGroupKeyNamed (Class|RealtimeMeshBlueprintFunctionLibrary|MakeLODKey) "Test") _builder_5))