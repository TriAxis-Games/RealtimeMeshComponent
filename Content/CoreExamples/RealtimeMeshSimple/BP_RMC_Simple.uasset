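; Example Realtime Mesh Component actor that procedurally builds a single two-sided triangle.
; On OnGenerateMesh, a local mesh builder fills a stream set with three colored vertices and two triangles of opposite winding, the second in its own poly group.
; A RealtimeMeshSimple turns the stream set into a unique LOD 0 section group and sets up red and blue material slots for the two sides.
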(event EventBeginPlay)

(event Collision|EventActorBeginOverlap
  (params (OtherActor :type Actor%20Object%20Reference)))

(event EventTick
  (params (DeltaSeconds :type Float%20%28single-precision%29)))

(event EventOnGenerateMesh
  (bind _returnvalue (Class|RealtimeMeshStreamUtils|MakeRealtimeMeshStreamSet))
  (bind _returnvalue_2 (Class|RealtimeMeshStreamUtils|MakeLocalMeshBuilder _returnvalue "Normal" "Normal" "Normal" "Normal" true 1 true))
  (bind _returnvalue_3 (Class|RealtimeMeshStreamUtils|AddVertex _returnvalue_2 "-50.000000,0.000000,0.000000" "0.000000,-1.000000,1.000000" "1.000000,0.000000,0.000000" "(R=1.000000,G=0.050353,B=0.000000,A=1.000000)" "(X=0.000000,Y=0.000000)" "(X=0.000000,Y=0.000000)" "(X=0.000000,Y=0.000000)" "(X=0.000000,Y=0.000000)"))
  (bind _returnvalue_4 (Class|RealtimeMeshStreamUtils|AddVertex _returnvalue_3 "0.000000,0.000000,100.000000" "0.000000,-1.000000,1.000000" "1.000000,0.000000,0.000000" "(R=0.000000,G=1.000000,B=0.106628,A=1.000000)" "(X=0.000000,Y=1.000000)" "(X=0.000000,Y=0.000000)" "(X=0.000000,Y=0.000000)" "(X=0.000000,Y=0.000000)"))
  (bind _returnvalue_5 (Class|RealtimeMeshStreamUtils|AddVertex _returnvalue_4 "50.000000,0.000000,0.000000" "0.000000,-1.000000,1.000000" "1.000000,0.000000,0.000000" "(R=0.000000,G=0.041400,B=1.000000,A=1.000000)" "(X=1.000000,Y=0.000000)" "(X=0.000000,Y=0.000000)" "(X=0.000000,Y=0.000000)" "(X=0.000000,Y=0.000000)"))
  (bind _returnvalue_6 (Class|RealtimeMeshStreamUtils|AddTriangle _returnvalue_5 0 1 2))
  (Class|RealtimeMeshStreamUtils|AddTriangle _returnvalue_6 2 1 0 1)
  (bind _returnvalue_7 (Class|RealtimeMeshComponent|InitializeRealtimeMesh (Variables|Default|GetRealtimeMeshComponent) "/Script/RealtimeMeshComponent.RealtimeMeshSimple"))
  (Class|RealtimeMeshSimple|CreateSectionGroup _returnvalue_7 (Class|RealtimeMeshBlueprintFunctionLibrary|MakeSectionGroupKeyUnique (Class|RealtimeMeshBlueprintFunctionLibrary|MakeLODKey)) _returnvalue)
  (Class|RealtimeMesh|SetupMaterialSlot _returnvalue_7 0 "None" "/AnimationSharing/AnimSharingRed.AnimSharingRed")
  (Class|RealtimeMesh|SetupMaterialSlot _returnvalue_7 1 "None" "/AnimationSharing/AnimSharingBlue.AnimSharingBlue"))

(fn ConstructionScript)